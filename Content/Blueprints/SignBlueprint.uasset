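; Sign actor that lets the player type a message, which is copied to its Message text.
; Input is off at BeginPlay and enabled on any actor overlap, so Interact can open a SignUI widget.
; After a short delay, a throttled Tick polls the text box's keyboard focus, printing a debug string while focused.
; Without focus, it removes the widget and applies the text; Tick is never switched off again.
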(event EventBeginPlay
  (Input|DisableInput (Game|GetPlayerController 0))
  (Actor|Tick|SetActorTickEnabled false)
  (Actor|Tick|SetActorTickInterval 0.1))

(event Collision|EventActorBeginOverlap
  (params (OtherActor :type Actor%20Object%20Reference))
  (Input|EnableInput (Game|GetPlayerController 0)))

(event EventTick
  (params (DeltaSeconds :type Float%20%28single-precision%29))
  (if (Class|Widget|HasKeyboardFocus (Variables|/Game/Blueprints/SignUI.SignUI_C|GetEditableTextBox_47 (stale Input|ActionEvents|InputActionInteract _returnvalue)))
    (Development|PrintString "HAS FOCUS")
    (else
      (Widget|RemovefromParent (stale Input|ActionEvents|InputActionInteract _returnvalue))
      (Rendering|Components|TextRender|SetText (Variables|Default|GetMessage) (Class|EditableTextBox|GetText (Variables|/Game/Blueprints/SignUI.SignUI_C|GetEditableTextBox_47 (stale Input|ActionEvents|InputActionInteract _returnvalue)))))))

(event Input|ActionEvents|InputActionInteract
  (params (Key :type Key%20Structure :default "None"))
  (:Pressed
    (bind _returnvalue (UserInterface|CreateWidget "/Game/Blueprints/SignUI.SignUI_C"))
    (UserInterface|Viewport|AddtoViewport _returnvalue 0)
    (Utilities|FlowControl|Delay 0.5)
    (Actor|Tick|SetActorTickEnabled true)))

(fn ConstructionScript)