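; Fireball projectile actor that launches forward on spawn and explodes on overlap.
; BeginPlay sets its mesh's physics velocity along the actor's forward vector, then destroys it after a timed lifespan.
; On overlap it enables physics on the other actor's static mesh, applies a radial velocity-change impulse to it and spawns an explosion emitter.
; A short delay then leads into the shared destroy step.
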(event EventBeginPlay
  (Physics|SetPhysicsLinearVelocity (Variables|Debug|GetStaticMeshComponent) (* (Math|Vector|GetForwardVector (Transformation|GetActorRotation)) 2e+03) false "None")
  (Transformation|SetMobility "Movable")
  (Utilities|FlowControl|Delay 1e+01)
  (Actor|DestroyActor))

(event Collision|EventActorBeginOverlap
  (params (OtherActor :type Actor%20Object%20Reference))
  (bind _returnvalue (Actor|GetComponentbyClass OtherActor "/Script/Engine.StaticMeshComponent"))
  (Physics|SetSimulatePhysics _returnvalue true)
  (Physics|AddRadialImpulse _returnvalue "0, 0, 0" 1e+04 3e+03 "RIF_Constant" true)
  (Effects|SpawnEmitteratLocation "/Game/Blueprints/Explosion.Explosion" (Transformation|GetActorLocation))
  (Utilities|FlowControl|Delay 0.2)
  (Actor|DestroyActor))

(event EventTick
  (params (DeltaSeconds :type Float%20%28single-precision%29)))

(fn ConstructionScript)