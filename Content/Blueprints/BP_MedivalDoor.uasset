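; BP_MedivalDoor is an interactive door actor that swings open and closed when the player presses Interact.
; A box collision enables input for player 0 on overlap and disables it on exit.
; Each press toggles a closed flag, swaps the open and close audio, and plays or reverses a timeline that drives the door's relative yaw.
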(event OnComponentBeginOverlap(BoxCollision)
  (params (OverlappedComponent :type Primitive%20Component%20Object%20Reference) (OtherActor :type Actor%20Object%20Reference) (OtherComp :type Primitive%20Component%20Object%20Reference) (OtherBodyIndex :type Integer) (bFromSweep :type Boolean) (SweepResult :type Hit%20Result%20Structure%20%28by%20ref%29))
  (Input|EnableInput (Game|GetPlayerController 0)))

(event OnComponentEndOverlap(BoxCollision)
  (params (OverlappedComponent :type Primitive%20Component%20Object%20Reference) (OtherActor :type Actor%20Object%20Reference) (OtherComp :type Primitive%20Component%20Object%20Reference) (OtherBodyIndex :type Integer))
  (Input|DisableInput (Game|GetPlayerController 0)))

(event EventBeginPlay)

(event Collision|EventActorBeginOverlap
  (params (OtherActor :type Actor%20Object%20Reference)))

(event Input|ActionEvents|InputActionInteract
  (params (Key :type Key%20Structure :default "None"))
  (:Pressed
    (if (Variables|Default|GetIsDoorClosed)
      (Audio|Components|Audio|Stop (Variables|Default|Getdoor_close))
      (Audio|Components|Audio|Play (Variables|Default|Getdoor_open) 0.0)
      (Variables|Default|SetIsDoorClosed false)
      (bind _dooranimation (Timeline|DoorAnimation Play)
        (:Update
          (Transformation|SetRelativeRotation (Variables|Default|GetDoor) (Math|Rotator|MakeRotator 0.0 0.0 _dooranimation) false false)))
      (else
        (Audio|Components|Audio|Stop (Variables|Default|Getdoor_open))
        (Audio|Components|Audio|Play (Variables|Default|Getdoor_close) 0.0)
        (Variables|Default|SetIsDoorClosed true)
        (Timeline|DoorAnimation Reverse)))))

(fn ConstructionScript)